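; Player character Blueprint that handles the basic weapon attack and owns the action bar HUD.
; It creates the HUD at startup, toggles it through events, and refreshes life, mana and jump-charge ratios every tick.
; Attack events switch weapon collision on and off.
; Weapon overlaps apply fixed damage, filtering out self, the Tower and, via a substring-index check, components named starting with "RangeAttack".
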(event `self.ReceiveBeginPlay`
  ;[1 1 1] DisableCollisionWeapon
  (`PrimitiveComponent.SetCollisionEnabled` (`self.WeaponCollision`) "NoCollision")
  ;[1 1 1] Add UI
  (bind _returnvalue (`|CreateWidget` "/Game/Core/UI/InGame/UMG_ActionBar_UserInterface.UMG_ActionBar_UserInterface_C"))
  (bind _output_get (set `self.PlayerUIRef` _returnvalue))
  (`UserWidget.AddToViewport` _output_get 0))

(event `self.ReceiveTick`
  (params (DeltaSeconds :type "Float (single-precision)"))
  (`self.UpdateUI`))

(event `ToggleHudOff`
  ;[1 1 1] Pause UI
  (`Widget.RemoveFromParent` (`self.PlayerUIRef`)))

(event `self.ReceiveBeginAttack`
  ;[1 1 1] Delegate
  (`PrimitiveComponent.SetCollisionEnabled` (`self.WeaponCollision`) "QueryOnly"))

(event `self.ReceiveEndAttack`
  ;[1 1 1] Delegate
  (`PrimitiveComponent.SetCollisionEnabled` (`self.WeaponCollision`) "NoCollision"))

(event `ToggleHudOn`
  ;[1 1 1] Pause UI
  (`UserWidget.AddToViewport` (`self.PlayerUIRef`) 0))

(event `self.WeaponCollision.OnComponentBeginOverlap`
  (params (OverlappedComponent :type "PrimitiveComponent Object Reference") (OtherActor :type "Actor Object Reference") (OtherComp :type "PrimitiveComponent Object Reference") (OtherBodyIndex :type Integer) (bFromSweep :type Boolean) (SweepResult :type "HitResult Structure (by ref)"))
  ;[1 1 1] BasicAttack
  (if (and (!= OtherActor (`self.Tower`)) (!= OtherActor self) (`KismetMathLibrary.Conv_IntToBool` (`KismetStringLibrary.FindSubstring` (`KismetSystemLibrary.GetDisplayName` OtherComp) "RangeAttack")))
    (`GameplayStatics.ApplyDamage` OtherActor 5.0 (`Pawn.GetController`) self)))

(fn `UpdateUI`
  (bind _playeruiref (`self.PlayerUIRef`))
  (`/Game/Core/UI/InGame/UMG_ActionBar_UserInterface.UpdateLife` (`self.PlayerUIRef`) (/ (`LifeComponent.Life` (`self.Life`)) (`self.InitLife`)))
  (`/Game/Core/UI/InGame/UMG_ActionBar_UserInterface.UpdateMana` _playeruiref (/ (`self.CurrentMana`) (`self.MaxMana`)))
  (`/Game/Core/UI/InGame/UMG_ActionBar_UserInterface.UpdateJump` _playeruiref (/ (`self.ElapseJump`) (`self.TimeChargeJump`))))

(fn `UserConstructionScript`)