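; Game mode Blueprint that runs the win and game-over flows and shows the minimap.
; BeginPlay creates the minimap widget, stores it and adds it to the viewport.
; OnGameOver and OnWinGame each show their end screen, then, if the player controller is valid, switch to UI-only input focused on the restart button, show the cursor, pause, hide the player HUD and play a lose or win sound.
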(event `self.OnGameOver`
  (bind _returnvalue (`GameplayStatics.GetPlayerController` 0))
  (bind _returnvalue_2 (`|CreateWidget` "/Game/Core/UI/OffGame/UMG_GameOverScreen.UMG_GameOverScreen_C"))
  (`UserWidget.AddToViewport` _returnvalue_2 0)
  (`/Engine/EditorBlueprintResources/StandardMacros.IsValid` _returnvalue
    (:`Is Valid`
      (`WidgetBlueprintLibrary.SetInputMode_UIOnlyEx` _returnvalue (`/Game/Core/UI/OffGame/UMG_Button.MyButton` (`/Game/Core/UI/OffGame/UMG_GameOverScreen.RestartGame` _returnvalue_2)))
      (set `PlayerController.bShowMouseCursor` true _returnvalue)
      (`GameplayStatics.SetGamePaused` true)
      (`/Game/Core/Player/PlayerCharacter_BP.ToggleHudOff` (cast `/Game/Core/Player/PlayerCharacter_BP` (`GameplayStatics.GetPlayerCharacter` 0) :!pure true))
      (bind _returnvalue_3 (`GameplayStatics.CreateSound2D` "/Game/Core/Audios/AudioOffGame/LoseGame_Sound.LoseGame_Sound" 1.0 1.0 0.0 null))
      (`AudioComponent.Play` _returnvalue_3 0.0))))

(event `self.OnWinGame`
  (bind _returnvalue (`GameplayStatics.GetPlayerController` 0))
  (bind _returnvalue_2 (`|CreateWidget` "/Game/Core/UI/OffGame/UMG_PlayerWin.UMG_PlayerWin_C"))
  (`UserWidget.AddToViewport` _returnvalue_2 0)
  (`/Engine/EditorBlueprintResources/StandardMacros.IsValid` _returnvalue
    (:`Is Valid`
      (`WidgetBlueprintLibrary.SetInputMode_UIOnlyEx` _returnvalue (`/Game/Core/UI/OffGame/UMG_Button.MyButton` (`/Game/Core/UI/OffGame/UMG_PlayerWin.RestartGame` _returnvalue_2)))
      (set `PlayerController.bShowMouseCursor` true _returnvalue)
      (`GameplayStatics.SetGamePaused` true)
      (`/Game/Core/Player/PlayerCharacter_BP.ToggleHudOff` (cast `/Game/Core/Player/PlayerCharacter_BP` (`GameplayStatics.GetPlayerCharacter` 0) :!pure true))
      (bind _returnvalue_3 (`GameplayStatics.CreateSound2D` "/Game/Core/Audios/AudioOffGame/WinGame_Sound.WinGame_Sound" 1.0 1.0 0.0 null))
      (`AudioComponent.Play` _returnvalue_3 0.0))))

(event `self.ReceiveBeginPlay`
  (bind _returnvalue (`|CreateWidget` "/Game/Core/MniMap/UMG_Minimap.UMG_Minimap_C"))
  (bind _output_get (set `self.MiniMap` _returnvalue))
  (`UserWidget.AddToViewport` _output_get 0))

(fn `UserConstructionScript`)