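; Slow enemy Blueprint that deals melee damage through a DamageZone and shows its life on a widget health bar.
; ABP_DogEnemy attack begin and end events toggle the zone's collision, so it only registers overlaps during attacks.
; Overlaps apply fixed damage to any actor that is not an EnemyCharacter.
; Tick pushes current life as a ratio of initial life to the health bar widget.
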(event `OnAttackBeginEvent`
  ;[1 1 1] SetEvent
  (`PrimitiveComponent.SetCollisionEnabled` (`self.DamageZone`) "QueryOnly"))

(event `self.ReceiveBeginPlay`
  ;[1 1 1] SetEvent
  (`PrimitiveComponent.SetCollisionEnabled` (`self.DamageZone`) "NoCollision")
  (bind _asabp_dog_enemy (cast `/Game/Core/Enemy/Animation/ABP_DogEnemy` (`SkeletalMeshComponent.GetAnimInstance` (`self.Mesh`))))
  (add `/Game/Core/Enemy/Animation/ABP_DogEnemy.OnAttackBegin` _asabp_dog_enemy (delegate `OnAttackBeginEvent`))
  (add `/Game/Core/Enemy/Animation/ABP_DogEnemy.OnAttackEnd` _asabp_dog_enemy (delegate `OnAttackEndEvent`)))

(event `OnAttackEndEvent`
  ;[1 1 1] SetEvent
  (`PrimitiveComponent.SetCollisionEnabled` (`self.DamageZone`) "NoCollision"))

(event `self.ReceiveTick`
  (params (DeltaSeconds :type "Float (single-precision)"))
  ;[1 1 1] UpdateLife
  (bind _asumg_display_enemy_life_lent (cast `/Game/Core/UI/InGame/UMG_Display_enemyLife_Lent` (`WidgetComponent.GetUserWidgetObject` (`self.HealthBar`))))
  (`/Game/Core/UI/InGame/UMG_Display_enemyLife_Lent.UpdateHeath` _asumg_display_enemy_life_lent (/ (`LifeComponent.Life` (`self.Life`)) (`self.InitLife`))))

(event `self.DamageZone.OnComponentBeginOverlap`
  (params (OverlappedComponent :type "PrimitiveComponent Object Reference") (OtherActor :type "Actor Object Reference") (OtherComp :type "PrimitiveComponent Object Reference") (OtherBodyIndex :type Integer) (bFromSweep :type Boolean) (SweepResult :type "HitResult Structure (by ref)"))
  ;[1 1 1] Apply Damage
  (cast `EnemyCharacter` OtherActor
    (:`CastFailed`
      (`GameplayStatics.ApplyDamage` OtherActor 5.0 (`self.GetController`) self))))

(fn `UserConstructionScript`)