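; PandaTower_BP is a tower actor that reports its remaining life to the player's UI.
; Every Tick it casts player 0's character to PlayerCharacter_BP and passes Life.Life divided by InitLife to UpdateTowerLife on that character's PlayerUIRef.
; An older path that updated a UMG_Display_TowerLife widget directly remains in the graph but never runs.
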(event `self.ReceiveTick`
  (params (DeltaSeconds :type "Float (single-precision)"))
  ;[1 1 1] Update Life
  (bind _asplayer_character_bp (cast `/Game/Core/Player/PlayerCharacter_BP` (`GameplayStatics.GetPlayerCharacter` 0)))
  (`/Game/Core/UI/InGame/UMG_ActionBar_UserInterface.UpdateTowerLife` (`/Game/Core/Player/PlayerCharacter_BP.PlayerUIRef` _asplayer_character_bp) (/ (`LifeComponent.Life` (`self.Life`)) (`self.InitLife`))))

(fn `UserConstructionScript`)